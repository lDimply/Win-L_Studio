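; Blueprint that tracks the level 2 star score for correct and incorrect results.
; On BeginPlay it creates and stores a WBP_EstrellasLVL2 widget, without adding it to the viewport here.
; The correct event increments both ActualEstrellasLVL2 and MaxEstrellasLVL2 on BP_FirstPersonGameMode, while the incorrect one raises only ActualEstrellasLVL2.
; Both then call the widget's star update with zero arguments and print a debug result.
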(event Custom|Agregar%20Estrellas%20Y%20Denominador%20LVL%202%20%28CORRECTO%29
  (bind _asbp_first_person_game_mode (Utilities|Casting|CastToBP_FirstPersonGameMode (Game|GetGameMode)))
  (Variables|/Game/FirstPerson/Blueprints/BP_FirstPersonGameMode.BP_FirstPersonGameMode_C|SetActualEstrellasLVL2 _asbp_first_person_game_mode (+ (Variables|/Game/FirstPerson/Blueprints/BP_FirstPersonGameMode.BP_FirstPersonGameMode_C|GetActualEstrellasLVL2 _asbp_first_person_game_mode) 1))
  (Variables|/Game/FirstPerson/Blueprints/BP_FirstPersonGameMode.BP_FirstPersonGameMode_C|SetMaxEstrellasLVL2 _asbp_first_person_game_mode (+ (Variables|/Game/FirstPerson/Blueprints/BP_FirstPersonGameMode.BP_FirstPersonGameMode_C|GetMaxEstrellasLVL2 _asbp_first_person_game_mode) 1))
  (Default|ACTUALIZARCANVAESTRELLAS (Variables|Default|GetWBP_EstrellaLVL2))
  (Development|PrintString "Correcto" true true "(R=0.000000,G=0.660000,B=1.000000,A=1.000000)" 5.0))

(event Custom|Agregar%20Denominador%20sin%20estrella%20LVL2%20INCORRECTO
  (bind _asbp_first_person_game_mode (Utilities|Casting|CastToBP_FirstPersonGameMode (Game|GetGameMode)))
  (Variables|/Game/FirstPerson/Blueprints/BP_FirstPersonGameMode.BP_FirstPersonGameMode_C|SetActualEstrellasLVL2 _asbp_first_person_game_mode (+ (Variables|/Game/FirstPerson/Blueprints/BP_FirstPersonGameMode.BP_FirstPersonGameMode_C|GetActualEstrellasLVL2 _asbp_first_person_game_mode) 1))
  (Variables|/Game/FirstPerson/Blueprints/BP_FirstPersonGameMode.BP_FirstPersonGameMode_C|SetMaxEstrellasLVL2 _asbp_first_person_game_mode (+ (Variables|/Game/FirstPerson/Blueprints/BP_FirstPersonGameMode.BP_FirstPersonGameMode_C|GetMaxEstrellasLVL2 _asbp_first_person_game_mode) 0))
  (Default|ACTUALIZARCANVAESTRELLAS (Variables|Default|GetWBP_EstrellaLVL2))
  (Development|PrintString "Incorrecto" true true "(R=0.000000,G=0.660000,B=1.000000,A=1.000000)" 5.0))

(event EventBeginPlay
  (bind _returnvalue (UserInterface|CreateWidget "/Game/2_UI/3_UI_Estrellas/WBP_EstrellasLVL2.WBP_EstrellasLVL2_C"))
  (Variables|Default|SetWBP_EstrellaLVL2 _returnvalue))

(fn ConstructionScript)