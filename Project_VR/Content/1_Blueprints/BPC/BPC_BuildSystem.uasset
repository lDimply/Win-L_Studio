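; VR building component that lets the player preview, place and destroy parts loaded from DT_BuildParts.
; In build mode, a per-tick right-hand raycast snaps a translucent-material preview mesh of the selected part to HotSpot targets, where placing spawns its Blueprint.
; Index changes clear the preview for rebuilding, and a left-hand raycast destroys Buildable actors.
; A looping timer handles rotate input, but its computed rotation is never applied.
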(event Custom|PreviewLoop
  (bind _raycast_right (Variables|Raycast|GetRaycast%20Right))
  (bind _returnvalue (Transformation|GetWorldTransform _raycast_right))
  (bind (_outhit _returnvalue_2) (Collision|LineTraceForObjects (.location _returnvalue) (+ (.location _returnvalue) (* (Math|Vector|GetForwardVector (.rotation _returnvalue)) 1.5e+03)) (Variables|Default|GetObject%20Types) false (Utilities|Array|MakeArray (Variables|Default|GetBP_Floor)) "ForOneFrame"))
  (if _returnvalue_2
    (if (Actor|ActorHasTag (.HitActor (Collision|BreakHitResult _outhit)) "HotSpot")
      (if (not (Actor|ActorHasTag (.HitActor (Collision|BreakHitResult _outhit)) "Buildable"))
        (Utilities|FlowControl|Sequence
          (:then_0
            (Utilities|FlowControl|DoOnce false
              (:Completed
                (bind _returnvalue_3 (Game|AddComponentbyClass (Variables|Default|GetAs%20VRPawn) "/Script/Engine.StaticMeshComponent" false (Variables|Default|GetBuild%20Preview%20Transform)))
                (bind _output_get (Variables|Default|SetPreviewMesh _returnvalue_3))
                (Components|StaticMesh|SetStaticMesh _output_get (.Mesh (Utilities|Struct|BreakS_BuildParts (Utilities|Array|Get(acopy) (Variables|Default|GetDT_Buildable) (Variables|Default|GetBuildable%20Index)))))
                (Rendering|Material|SetMaterial (Variables|Default|GetPreviewMesh) 0 "/Game/3_Materiales/BuildPreview/M_MaterialPreview.M_MaterialPreview")
                (Collision|SetCollisionEnabled (Variables|Default|GetPreviewMesh) "NoCollision"))))
          (:then_1
            (bind _output_get_2 (Variables|Default|SetBuild%20Preview%20Transform (Math|Transform|MakeTransform (Transformation|GetWorldLocation (.HitComponent (Collision|BreakHitResult _outhit))) (Transformation|GetWorldRotation (.HitComponent (Collision|BreakHitResult _outhit))) "1.000000,1.000000,1.000000")))
            (Transformation|SetWorldTransform (Variables|Default|GetPreviewMesh) _output_get_2 false false)))))))

(event Custom|Reset%20Build%20Mode
  (Utilities|FlowControl|DoOnce false) ; enters at Reset
)

(event Custom|Stop%20Build%20Mode
  (Variables|Default|SetinBuildMode false)
  (bind _previewmesh (Variables|Default|GetPreviewMesh)
    (:then
      (Components|StaticMesh|SetStaticMesh _previewmesh 0)
      (Variables|Default|SetPreviewMesh 0)
      (CallFunction|ResetBuildMode))
    (:else)))

(event Custom|Rotate%20Preview
  (Variables|Default|SetBuildPreviewRotation (Math|Rotator|CombineRotators (.rotation (Variables|Default|GetBuild%20Preview%20Transform)) "0.000000,5.000000,0.000000")))

(event Custom|IncreseaBuildIndex
  (Variables|Default|SetBuildable%20Index (Math|Integer|Clamp(Integer) (+ (Variables|Default|GetBuildable%20Index) 1) 0 (- (Utilities|Array|Length (Variables|Default|GetDT_Buildable)) 1)))
  (bind _previewmesh (Variables|Default|GetPreviewMesh)
    (:then
      (Components|StaticMesh|SetStaticMesh _previewmesh 0)
      (Variables|Default|SetPreviewMesh 0)
      (CallFunction|ResetBuildMode))
    (:else)))

(event Custom|DecrementBuildIndex
  (Variables|Default|SetBuildable%20Index (Math|Integer|Clamp(Integer) (- (Variables|Default|GetBuildable%20Index) 1) 0 (- (Utilities|Array|Length (Variables|Default|GetDT_Buildable)) 1)))
  (bind _previewmesh (Variables|Default|GetPreviewMesh)
    (:then
      (Components|StaticMesh|SetStaticMesh _previewmesh 0)
      (Variables|Default|SetPreviewMesh 0)
      (CallFunction|ResetBuildMode))
    (:else)))

(event Input|EnhancedActionEvents|EnhancedInputActionIA_Build
  (params (ActionValue :type Boolean) (ElapsedSeconds :type Float%20%28double-precision%29) (TriggeredSeconds :type Float%20%28double-precision%29) (InputAction :type Input%20Action%20Object%20Reference :default "/Game/1_Blueprints/Inputs/IA_Build.IA_Build"))
  (:Started
    (if (not (Variables|Default|GetinBuildMode))
      (Variables|Default|SetinBuildMode true)
      (else
        (Variables|Default|SetinBuildMode false)
        (bind _previewmesh (Variables|Default|GetPreviewMesh)
          (:then
            (Components|StaticMesh|SetStaticMesh _previewmesh 0)
            (Variables|Default|SetPreviewMesh 0)
            (CallFunction|ResetBuildMode))
          (:else))))))

(event Input|EnhancedActionEvents|EnhancedInputActionIA_PlaceBuild
  (params (ActionValue :type Boolean) (ElapsedSeconds :type Float%20%28double-precision%29) (TriggeredSeconds :type Float%20%28double-precision%29) (InputAction :type Input%20Action%20Object%20Reference :default "/Game/1_Blueprints/Inputs/IA_PlaceBuild.IA_PlaceBuild"))
  (:Started
    (if (Variables|Default|GetinBuildMode)
      (Game|SpawnActorfromClass (.Blueprint (Utilities|Struct|BreakS_BuildParts (Utilities|Array|Get(acopy) (Variables|Default|GetDT_Buildable) (Variables|Default|GetBuildable%20Index)))) (Variables|Default|GetBuild%20Preview%20Transform) "AlwaysSpawn" "MultiplyWithRoot" 0 0)
      (CallFunction|StopBuildMode))))

(event Input|EnhancedActionEvents|EnhancedInputActionIA_RotateBuild
  (params (ActionValue :type Boolean) (ElapsedSeconds :type Float%20%28double-precision%29) (TriggeredSeconds :type Float%20%28double-precision%29) (InputAction :type Input%20Action%20Object%20Reference :default "/Game/1_Blueprints/Inputs/IA_RotateBuild.IA_RotateBuild"))
  (:Started
    (bind _returnvalue (Utilities|Time|SetTimerbyEvent (delegate Custom|Rotate%20Preview) 0.1 true))
    (Variables|Default|SetRotate%20Build%20Preview%20Loop _returnvalue))
  (:Completed
    (Utilities|Time|ClearandInvalidateTimerbyHandle (Variables|Default|GetRotate%20Build%20Preview%20Loop))
    (Variables|Default|SetRotate%20Build%20Preview%20Loop "")))

(event Input|EnhancedActionEvents|EnhancedInputActionIA_TriggerInteracction
  (params (ActionValue :type Boolean) (ElapsedSeconds :type Float%20%28double-precision%29) (TriggeredSeconds :type Float%20%28double-precision%29) (InputAction :type Input%20Action%20Object%20Reference :default "/Game/1_Blueprints/Inputs/IA_TriggerInteracction.IA_TriggerInteracction"))
  (bind _raycast_left (Variables|Raycast|GetRaycast%20Left))
  (bind _returnvalue (Transformation|GetWorldTransform _raycast_left))
  (:Started
    (bind (_outhit _returnvalue_2) (Collision|LineTraceByChannel (.location _returnvalue) (+ (.location _returnvalue) (* (Math|Vector|GetForwardVector (.rotation _returnvalue)) 1.5e+03)) "TraceTypeQuery1" false 0 "None"))
    (if _returnvalue_2
      (if (Actor|ActorHasTag (.HitActor (Collision|BreakHitResult _outhit)) "Buildable")
        (Actor|DestroyActor (.HitActor (Collision|BreakHitResult _outhit)))))))

(event EventTick
  (params (DeltaSeconds :type Float%20%28single-precision%29))
  (if (Variables|Default|GetinBuildMode)
    (CallFunction|PreviewLoop)))

(event EventBeginPlay
  (bind _asvrpawn (Utilities|Casting|CastToVRPawn (Game|Player|GetPlayerPawn 0)))
  (Variables|Raycast|SetRaycast%20Right (Variables|/Game/VRTemplate/Blueprints/VRPawn.VRPawn_C|GetRaycastRight _asvrpawn))
  (Variables|Raycast|SetRaycast%20Left (Variables|/Game/VRTemplate/Blueprints/VRPawn.VRPawn_C|GetRaycastLeft _asvrpawn))
  (Variables|Default|SetAs%20VRPawn _asvrpawn)
  (bind _returnvalue (Actor|GetActorOfClass "/Game/1_Blueprints/Actors/1_BuildMaster/BP_Floor.BP_Floor_C"))
  (Variables|Default|SetBP_Floor _returnvalue)
  (bind _outrownames (DataTable|GetDataTableRowNames "/Game/1_Blueprints/DataBase/1_BuldPartDatabase/DT_BuildParts.DT_BuildParts"))
  (for _array_element _outrownames
    (bind _returnvalue_2 (Utilities|GetDataTableRow "/Game/1_Blueprints/DataBase/1_BuldPartDatabase/DT_BuildParts.DT_BuildParts" _array_element)
      (:then
        (Utilities|Array|Add (Variables|Default|GetDT_Buildable) _returnvalue_2)))))