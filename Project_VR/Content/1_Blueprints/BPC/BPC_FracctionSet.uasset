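; BPC_FracctionSet is a Blueprint component that runs a VR minigame comparing two fractions.
; On BeginPlay it caches the left and right fraction widgets from the VRPawn, then generates random fractions sharing a denominator, recursively rerolling when they are equal.
; It displays both and flags the larger side.
; FraccionComparacion checks the left/right input against that flag and prints a win or lose message.
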(event Custom|RANDOMGENERATION
  ;[1 1 1] Denominador
  (bind _output_get (Variables|Default|SetDenominadorFRAC1 (Math|Conversions|ToFloat(Integer) (Math|Random|RandomIntegerinRange 1 5))))
  (bind _output_get_2 (Variables|Default|SetDenominadorRAC2 _output_get))
  (Variables|Default|SetNumeradorFRAC1 (Math|Conversions|ToFloat(Integer) (Math|Random|RandomIntegerinRange 0 (Math|Float|Truncate _output_get_2))))
  (Variables|Default|SetNumeradorFRAC2 (Math|Conversions|ToFloat(Integer) (Math|Random|RandomIntegerinRange 0 (Math|Float|Truncate _output_get_2))))
  (Variables|Default|SetResultadoIzquierda (/ (Variables|Default|GetNumeradorFRAC1) (Variables|Default|GetDenominadorFRAC1)))
  (Variables|Default|SetResultadoDerecha (/ (Variables|Default|GetNumeradorFRAC2) (Variables|Default|GetDenominadorRAC2)))
  (if (== (Variables|Default|GetResultadoIzquierda) (Variables|Default|GetResultadoDerecha))
    (CallFunction|RANDOMGENERATION)
    (else
      (Default|SETNUMERADORYDENOMINADOR1 (Variables|Default|GetAs%20WBP%20Fraccion%20Left) (Variables|Default|GetNumeradorFRAC1) (Variables|Default|GetDenominadorFRAC1))
      (Default|SETNUMERADORYDENOMINADOR2 (Variables|Default|GetAs%20WBP%20Fraccion%20RIght) (Variables|Default|GetNumeradorFRAC2) (Variables|Default|GetDenominadorRAC2))
      (if (> (Variables|Default|GetResultadoIzquierda) (Variables|Default|GetResultadoDerecha))
        (Variables|Default|SetIzqMayor true)
        (Variables|Default|SetDerMayor false)
        (else
          (Variables|Default|SetDerMayor true)
          (Variables|Default|SetIzqMayor false))))))

(event Custom|FraccionComparacion
  (params (IzqInput :type Boolean) (DerInput :type Boolean))
  (if (Variables|Default|GetIzqMayor)
    (if IzqInput
      (Development|PrintString "Ganaste" true true "(R=0.000000,G=0.660000,B=1.000000,A=1.000000)" 1e+01)
      (else
        (Development|PrintString "Perdiste" true true "(R=0.000000,G=0.660000,B=1.000000,A=1.000000)" 1e+01)))
    (elif DerInput
      (Development|PrintString "Ganaste" true true "(R=0.000000,G=0.660000,B=1.000000,A=1.000000)" 1e+01)
      (else
        (Development|PrintString "Perdiste" true true "(R=0.000000,G=0.660000,B=1.000000,A=1.000000)" 1e+01)))))

(event EventBeginPlay
  (bind _asvrpawn (Utilities|Casting|CastToVRPawn (Game|Player|GetPlayerPawn 0)))
  (bind _aswbp_fraccion_left (Utilities|Casting|CastToWBP_FraccionLeft (UserInterface|GetWidget (Variables|/Game/VRTemplate/Blueprints/VRPawn.VRPawn_C|GetWidgetFraccionLeft _asvrpawn))))
  (Variables|Default|SetAs%20WBP%20Fraccion%20Left _aswbp_fraccion_left)
  (bind _aswbp_fraccion_right (Utilities|Casting|CastToWBP_FraccionRIght (UserInterface|GetWidget (Variables|/Game/VRTemplate/Blueprints/VRPawn.VRPawn_C|GetWidgetFraccionRight _asvrpawn))))
  (Variables|Default|SetAs%20WBP%20Fraccion%20RIght _aswbp_fraccion_right)
  (CallFunction|RANDOMGENERATION))