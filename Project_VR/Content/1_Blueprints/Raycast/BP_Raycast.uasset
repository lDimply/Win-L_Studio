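; BP_Raycast lets the VR player interact with objects by pointing a short ray from the pawn's right-side raycast component.
; BeginPlay caches the player's VRPawn.
; The trigger interaction input line-traces forward from RaycastRight on the Visibility channel, with debug drawing enabled.
; A hit actor implementing BPI_Interactable receives InteractMessage, so targets define their own response through the interface.
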(event Input|EnhancedActionEvents|EnhancedInputActionIA_TriggerInteracction
  (params (ActionValue :type Boolean) (ElapsedSeconds :type Float%20%28double-precision%29) (TriggeredSeconds :type Float%20%28double-precision%29) (InputAction :type Input%20Action%20Object%20Reference :default "/Game/1_Blueprints/Inputs/IA_TriggerInteracction.IA_TriggerInteracction"))
  (bind _as_vrpawn (Variables|Default|GetAs%20VRPawn))
  (bind _raycastright (Variables|/Game/VRTemplate/Blueprints/VRPawn.VRPawn_C|GetRaycastRight _as_vrpawn))
  (bind _returnvalue (Transformation|GetWorldLocation _raycastright))
  (bind (_outhit _returnvalue_2) (Collision|LineTraceByChannel _returnvalue (+ _returnvalue (* (Math|Vector|GetForwardVector (Transformation|GetWorldRotation _raycastright)) 1.5e+02)) "TraceTypeQuery1" false 0 "ForOneFrame"))
  (if _returnvalue_2
    (if (Utilities|DoesObjectImplementInterface (.HitActor (Collision|BreakHitResult _outhit)) "/Game/1_Blueprints/BPI/BPI_Interactable.BPI_Interactable_C")
      (Class|BPIInteractable|Interact(Message) (.HitActor (Collision|BreakHitResult _outhit))))))

(event EventBeginPlay
  (Utilities|FlowControl|Sequence
    (:then_0
      (bind _asvrpawn (Utilities|Casting|CastToVRPawn (Game|Player|GetPlayerPawn 0)))
      (Variables|Default|SetAs%20VRPawn _asvrpawn))))