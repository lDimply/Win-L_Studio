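; BP_FraccionManager generates a pair of random fractions for a comparison puzzle and records which side is larger.
; On BeginPlay it creates and stores the left and right fraction widgets, without adding them to the viewport, then runs the generator.
; RANDOMGENFRACTION rolls two numerators over a shared denominator, recursively rerolling equal values.
; It passes valid pairs to the widgets, sets IzqMayor or DerMayor, and prints the larger side.
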(event Custom|RANDOMGENFRACTION
  ;[1 1 1] Denominador
  (bind _output_get (Variables|Default|SetDenominadorFRAC1 (Math|Conversions|ToFloat(Integer) (Math|Random|RandomIntegerinRange 1 5))))
  (bind _output_get_2 (Variables|Default|SetDenominadorRAC2 _output_get))
  (Variables|Default|SetNumeradorFRAC1 (Math|Conversions|ToFloat(Integer) (Math|Random|RandomIntegerinRange 0 (Math|Float|Truncate _output_get_2))))
  (Variables|Default|SetNumeradorFRAC2 (Math|Conversions|ToFloat(Integer) (Math|Random|RandomIntegerinRange 0 (Math|Float|Truncate _output_get_2))))
  (Variables|Default|SetResultadoFrac1 (/ (Variables|Default|GetNumeradorFRAC1) (Variables|Default|GetDenominadorFRAC1)))
  (Variables|Default|SetResultadoFrac2 (/ (Variables|Default|GetNumeradorFRAC2) (Variables|Default|GetDenominadorRAC2)))
  (if (== (Variables|Default|GetResultadoFrac1) (Variables|Default|GetResultadoFrac2))
    (CallFunction|RANDOMGENFRACTION)
    (else
      (Default|SETNUMERADORYDENOMINADOR (Variables|Default|GetLeftFractionREF) (Variables|Default|GetNumeradorFRAC1) (Variables|Default|GetDenominadorFRAC1))
      (Default|SETNUMERADORYDENOMINADOR (Variables|Default|GetRightFractionREF) (Variables|Default|GetNumeradorFRAC2) (Variables|Default|GetDenominadorRAC2))
      (if (> (Variables|Default|GetResultadoFrac1) (Variables|Default|GetResultadoFrac2))
        (Variables|Default|SetIzqMayor true)
        (Variables|Default|SetDerMayor false)
        (Development|PrintString "IzqMayor")
        (else
          (Variables|Default|SetDerMayor true)
          (Variables|Default|SetIzqMayor false)
          (Development|PrintString "DerMayor"))))))

(event EventBeginPlay
  (bind _returnvalue (UserInterface|CreateWidget "/Game/2_UI/ComparacionFracciones/WBP_FraccionLeft.WBP_FraccionLeft_C"))
  (Variables|Default|SetLeftFractionREF _returnvalue)
  (bind _returnvalue_2 (UserInterface|CreateWidget "/Game/2_UI/ComparacionFracciones/WBP_FraccionRIght.WBP_FraccionRIght_C"))
  (Variables|Default|SetRightFractionREF _returnvalue_2)
  (CallFunction|RANDOMGENFRACTION))

(fn ConstructionScript)