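; BP_PuzzleLogic_Bridge drives the fraction bridge puzzle display, tracking the numerator shown on a widget.
; On BeginPlay it caches the WBP_Puente_Fracciones widget from its widget component and the first-person game mode.
; The ACTUALIZAR_PUENTE_WIDGET event adds a delta to the game mode's NumFracPuente, clamps it to a small range, and writes it to the widget's numerator text.
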(event Custom|ACTUALIZAR_PUENTE_WIDGET
  (params (Numerador :type Integer))
  (bind _output_get (Variables|/Game/FirstPerson/Blueprints/BP_FirstPersonGameMode.BP_FirstPersonGameMode_C|SetNumFracPuente (Variables|Default|GetBP_GameMode) (Math|Integer|Clamp(Integer) (+ Numerador (Variables|/Game/FirstPerson/Blueprints/BP_FirstPersonGameMode.BP_FirstPersonGameMode_C|GetNumFracPuente (Variables|Default|GetBP_GameMode))) 0 3)))
  (Rendering|Components|TextRender|SetText (Variables|/Game/2_UI/UI_Bote/WBP_Puente_Fracciones.WBP_Puente_Fracciones_C|GetNumerador (Variables|Default|GetAs%20WBP%20Puente%20Fracciones_0)) (Utilities|Text|ToText(Integer) _output_get)))

(event EventBeginPlay
  (bind _aswbp_puente_fracciones (Utilities|Casting|CastToWBP_Puente_Fracciones (UserInterface|GetWidget (Variables|Default|GetWidget))))
  (Variables|Default|SetAs%20WBP%20Puente%20Fracciones_0 _aswbp_puente_fracciones)
  (bind _asbp_first_person_game_mode (Utilities|Casting|CastToBP_FirstPersonGameMode (Game|GetGameMode)))
  (Variables|Default|SetBP_GameMode _asbp_first_person_game_mode))

(fn ConstructionScript
  (|CallParentFunction))