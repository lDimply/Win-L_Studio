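; Puzzle logic Blueprint that tracks fraction numerators for the boat and bridge puzzles and shows them on a WBP_BoteFracciones widget.
; On BeginPlay it reads both starting counts from BP_FirstPersonGameMode and caches the widget's numerator text.
; Separate events add to each count, clamp it to 0–3 and write to that same text.
; Only a full boat count triggers the widget's next-level reveal animation.
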(event Custom|NumeratorAddBote
  (params (num :type Integer))
  (bind _output_get (Variables|Default|SetNum%20Frac%20Barco (Math|Integer|Clamp(Integer) (+ num (Variables|Default|GetNum%20Frac%20Barco)) 0 3)))
  (Variables|/Script/UMG.TextBlock|SetText (Variables|Default|GetNumeradorWidgetText) (Utilities|Text|ToText(Integer) _output_get))
  (if (== (Variables|Default|GetNum%20Frac%20Barco) 3)
    (Default|FUNCIONANIMACIONAPARECERSIGUIENTENIVEL (Variables|Default|GetAs%20WBP%20Bote%20Fracciones))))

(event Custom|NumeradorAddPuente
  (params (Num :type Integer))
  (bind _output_get (Variables|Default|SetNum%20Frac%20Puente (Math|Integer|Clamp(Integer) (+ Num (Variables|Default|GetNum%20Frac%20Puente)) 0 3)))
  (Variables|/Script/UMG.TextBlock|SetText (Variables|Default|GetNumeradorWidgetText) (Utilities|Text|ToText(Integer) _output_get)))

(event EventBeginPlay
  (bind _asbp_first_person_game_mode (Utilities|Casting|CastToBP_FirstPersonGameMode (Game|GetGameMode)))
  (Variables|Default|SetNum%20Frac%20Barco (Variables|/Game/FirstPerson/Blueprints/BP_FirstPersonGameMode.BP_FirstPersonGameMode_C|GetNumFracBarco _asbp_first_person_game_mode))
  (Variables|Default|SetNum%20Frac%20Puente (Variables|/Game/FirstPerson/Blueprints/BP_FirstPersonGameMode.BP_FirstPersonGameMode_C|GetNumFracPuente _asbp_first_person_game_mode))
  (bind _aswbp_bote_fracciones (Utilities|Casting|CastToWBP_BoteFracciones (UserInterface|GetWidget (Variables|Default|GetWidget))))
  (Variables|Default|SetAs%20WBP%20Bote%20Fracciones _aswbp_bote_fracciones)
  (Variables|Default|SetNumeradorWidgetText (Variables|/Game/2_UI/UI_Bote/WBP_BoteFracciones.WBP_BoteFracciones_C|GetNumerador _aswbp_bote_fracciones)))

(fn ConstructionScript)